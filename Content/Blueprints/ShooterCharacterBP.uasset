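; Shooter character Blueprint that connects character state to the third-person hero animation Blueprint and HUD.
; BeginPlay creates crosshair and health indicator widgets, shown only for the locally controlled player, and caches the AnimBP.
; Tick feeds it zoom, reload, death and wrap-corrected view pitch, and lowers walk speed while zooming.
; The Fire event briefly pulses the animation's fire flag, only while moving on ground.
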(event `self.ReceiveBeginPlay`
  (bind _returnvalue (`SkeletalMeshComponent.GetAnimInstance` (`self.Mesh`)))
  (`parent.ReceiveBeginPlay`)
  (`|ExecutionSequence`
    (:`then_0`
      (bind _returnvalue_2 (`|CreateWidget` "/Game/UI/Crosshair.Crosshair_C"))
      (if (`self.IsLocallyControlled`)
        (`UserWidget.AddToViewport` _returnvalue_2 0))
      (`/Engine/EditorBlueprintResources/StandardMacros.IsValid` _returnvalue
        (:`Is Valid`
          (bind _asue4asp_hero_tpp_anim_blueprint (cast `/Game/AnimStarterPack/UE4ASP_HeroTPP_AnimBlueprint` _returnvalue))
          (set `self.AnimBP` _asue4asp_hero_tpp_anim_blueprint))))
    (:`then_1`
      (bind _returnvalue_3 (`|CreateWidget` "/Game/UI/WBP_HealthIndicator.WBP_HealthIndicator_C"))
      (if (`self.IsLocallyControlled`)
        (`UserWidget.AddToViewport` _returnvalue_3 0)))))

(event `self.ReceiveTick`
  (params (DeltaSeconds :type "Float (single-precision)"))
  (bind (_outlocation _outrotation) (`self.GetActorEyesViewPoint`))
  (bind _animbp (`self.AnimBP`))
  (`parent.ReceiveTick` DeltaSeconds)
  (set `/Game/AnimStarterPack/UE4ASP_HeroTPP_AnimBlueprint.IronSights` (`self.bWantsToZoom`) _animbp)
  (set `/Game/AnimStarterPack/UE4ASP_HeroTPP_AnimBlueprint.Pitch` (`KismetMathLibrary.SelectFloat` (- (.pitch _outrotation) 270.0) (+ (.pitch _outrotation) 90.0) (> (.pitch _outrotation) 270.0)) _animbp)
  (set `CharacterMovementComponent.MaxWalkSpeed` (`KismetMathLibrary.SelectFloat` 300.0 600.0 (`self.bWantsToZoom`)) (`self.CharacterMovement`))
  (set `/Game/AnimStarterPack/UE4ASP_HeroTPP_AnimBlueprint.ReloadingWeapon` (`self.bIsReloadingWeapon`) (`self.AnimBP`))
  (set `/Game/AnimStarterPack/UE4ASP_HeroTPP_AnimBlueprint.Died` (`self.bDied`) (`self.AnimBP`)))

(event `Fire`
  (bind _animbp (`self.AnimBP`))
  (if (`NavMovementComponent.IsMovingOnGround` (`self.CharacterMovement`))
    (set `/Game/AnimStarterPack/UE4ASP_HeroTPP_AnimBlueprint.Fire` true _animbp)
    (`KismetSystemLibrary.Delay` 0.1)
    (set `/Game/AnimStarterPack/UE4ASP_HeroTPP_AnimBlueprint.Fire` false _animbp)))

(fn `UserConstructionScript`)