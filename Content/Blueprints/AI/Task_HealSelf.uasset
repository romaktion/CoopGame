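; Behavior Tree task that lets a BP_AdvancedAI pawn heal itself to full health over time.
; On execute it caches the pawn's ShooterHealthComponent and starts a looping one-second timer, aborting if the cast or component lookup fails.
; The HealSelf event restores a fixed amount per tick, then clears the timer and finishes successfully once health reaches maximum.
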(event `self.ReceiveExecuteAI`
  (params (OwnerController :type "AIController Object Reference") (ControlledPawn :type "Pawn Object Reference"))
  (bind _asbp_advanced_ai (cast `/Game/Blueprints/AI/BP_AdvancedAI` ControlledPawn)
    (:`then`
      (bind _returnvalue (`Actor.GetComponentByClass` _asbp_advanced_ai "/Script/CoopGame.ShooterHealthComponent"))
      (`/Engine/EditorBlueprintResources/StandardMacros.IsValid` _returnvalue
        (:`Is Valid`
          (set `self.HC` _returnvalue)
          (bind _returnvalue_2 (`KismetSystemLibrary.K2_SetTimerDelegate` (`|CreateDelegate` :!event `HealSelf`) 1.0 true))
          (set `self.HealSelfTimerHandle` _returnvalue_2))
        (:`Is Not Valid`
          (`self.FinishAbort` :!label _label))))
    (:`CastFailed`
      (goto _label))))

(event `HealSelf`
  (bind _hc (`self.HC`))
  (bind _healselftimerhandle (`self.HealSelfTimerHandle`))
  (`ShooterHealthComponent.Heal` _hc 20.0)
  (if (>= (`ShooterHealthComponent.GetHealth` _hc) (`ShooterHealthComponent.GetMaxHealth` _hc))
    (`KismetSystemLibrary.K2_PauseTimerHandle` _healselftimerhandle)
    (`KismetSystemLibrary.K2_ClearAndInvalidateTimerHandle` _healselftimerhandle)
    (`self.FinishExecute` true)))