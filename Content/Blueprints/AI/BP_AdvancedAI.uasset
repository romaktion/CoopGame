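; AI-controlled character Blueprint that runs the BT_AdvancedAI behavior tree and signals its death to animation.
; On BeginPlay it calls the parent, caches the mesh's UE4ASP_HeroTPP_AnimBlueprint, then starts the tree if an AI controller is valid.
; A failed anim Blueprint cast also prevents the tree from starting.
; HealthComp's health-change event sets the anim Blueprint's Died flag once health reaches zero or below.
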(event `self.ReceiveBeginPlay`
  (bind _returnvalue (`AIBlueprintHelperLibrary.GetAIController` self))
  (`parent.ReceiveBeginPlay`)
  (bind _asue4asp_hero_tpp_anim_blueprint (cast `/Game/AnimStarterPack/UE4ASP_HeroTPP_AnimBlueprint` (`SkeletalMeshComponent.GetAnimInstance` (`self.Mesh`))))
  (set `self.AnimBP` _asue4asp_hero_tpp_anim_blueprint)
  (`/Engine/EditorBlueprintResources/StandardMacros.IsValid` _returnvalue
    (:`Is Valid`
      (`AIController.RunBehaviorTree` _returnvalue "/Game/Blueprints/AI/BT_AdvancedAI.BT_AdvancedAI"))))

(event `self.HealthComp.OnHeathChangedEvent`
  (params (HealthComp :type "ShooterHealthComponent Object Reference") (Health :type "Float (single-precision)") (HealthDelta :type "Float (single-precision)") (DamageType :type "DamageType Object Reference") (InstigatedBy :type "Controller Object Reference") (DamageCauser :type "Actor Object Reference"))
  (if (<= Health 0.0)
    (set `/Game/AnimStarterPack/UE4ASP_HeroTPP_AnimBlueprint.Died` true (`self.AnimBP`))))

(fn `UserConstructionScript`)