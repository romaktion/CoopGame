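; Behavior Tree decorator that passes when the AI-controlled pawn is within a maximum distance of a target actor.
; It reads the target actor from a configurable Blackboard key and compares the straight-line distance between their locations to MaxDistance.
; The check fails when the key holds no valid actor.
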(fn `PerformConditionCheckAI`
  (params (OwnerController :type "AIController Object Reference") (ControlledPawn :type "Pawn Object Reference"))
  (returns (ReturnValue :type Boolean))
  (bind _returnvalue (`BTFunctionLibrary.GetBlackboardValueAsActor` (`self.BlackBoardKey`)))
  (`/Engine/EditorBlueprintResources/StandardMacros.IsValid` _returnvalue
    (:`Is Valid`
      (return (<= (`KismetMathLibrary.VSize` (- (`Actor.K2_GetActorLocation` ControlledPawn) (`Actor.K2_GetActorLocation` _returnvalue))) (`self.MaxDistance`))))
    (:`Is Not Valid`
      (return false))))