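; A target dummy that ragdolls when its health runs out.
; The ShooterHealth component's health-change event, handled only on the authority, sets a replicated death flag once health reaches zero.
; The flag's RepNotify turns on physics simulation for all skeletal mesh bodies and makes the mesh ignore the physics body and pawn collision channels.
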(event `self.ShooterHealth.OnHeathChangedEvent`
  (params (HealthComp :type "ShooterHealthComponent Object Reference") (Health :type "Float (single-precision)") (HealthDelta :type "Float (single-precision)") (DamageType :type "DamageType Object Reference") (InstigatedBy :type "Controller Object Reference") (DamageCauser :type "Actor Object Reference"))
  (`/Engine/EditorBlueprintResources/ActorMacros.Switch Has Authority`
    (:`Authority`
      (if (<= Health 0.0)
        (`/Engine/EditorBlueprintResources/StandardMacros.DoOnce` false
          (:`Completed`
            (set `self.DeathRep` true)))))))

(fn `OnRep_DeathRep`
  (bind _skeletalmesh (`self.SkeletalMesh`))
  (if (`self.DeathRep`)
    (`SkeletalMeshComponent.SetAllBodiesSimulatePhysics` _skeletalmesh true)
    (`PrimitiveComponent.SetCollisionResponseToChannel` _skeletalmesh "ECC_PhysicsBody" "ECR_Ignore")
    (`PrimitiveComponent.SetCollisionResponseToChannel` _skeletalmesh "ECC_Pawn" "ECR_Ignore")))

(fn `UserConstructionScript`)